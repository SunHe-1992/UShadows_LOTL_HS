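; BP_KnightPrisoner is a prisoner character that loops an idle animation on its skeletal mesh from BeginPlay.
; Interact casts the instigator's player state to US_PlayerState, awards EarnedXp, plays a one-shot cheer animation and prints a debug string.
; CanInteract always returns false, and the cheer does not switch back to the idle loop.
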(event `self.ReceiveBeginPlay`
  (`SkeletalMeshComponent.PlayAnimation` (`self.SkeletalMesh`) (`self.MontageIdle`) true))

(event `CharacterCheer`
  (`SkeletalMeshComponent.PlayAnimation` (`self.SkeletalMesh`) (`self.MontageCheer`) false))

(event `self.Interact`
  (params (CharacterInstigator :type "US_Character Object Reference"))
  (bind _asus_player_state (cast `US_PlayerState` (`Pawn.PlayerState` CharacterInstigator)))
  (`US_PlayerState.AddXp` _asus_player_state (`self.EarnedXp`))
  (`self.CharacterCheer`)
  (`KismetSystemLibrary.PrintString` "prisoner interact"))

(fn `CanInteract`
  (params (CharacterInstigator :type "US_Character Object Reference"))
  (returns (ReturnValue :type Boolean))
  (return false))

(fn `UserConstructionScript`)